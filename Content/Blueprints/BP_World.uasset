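; BP_World drives random battle encounters while its overlap flag is set through the Overlapping and StopOverlapping events.
; Each Tick with the flag on makes two chained random rolls to decide whether combat starts.
; On success it fills the three enemy slots in Instance_Game with random picks from the first two CurrentEnemies entries, then opens the Minimal_Default level after a short delay.
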(event `self.ReceiveBeginPlay`)

(event `self.ReceiveTick`
  (params (DeltaSeconds :type "Float (single-precision)"))
  (if (`self.Overlap`)
    (`self.Enable Combat`)))

(event `/Game/Blueprints/BP_Interface.Overlapping`
  ;[1 1 1] SetOverlapping
  (`KismetSystemLibrary.PrintString` "This is BP_World Starting")
  (set `self.Overlap` true))

(event `/Game/Blueprints/BP_Interface.StopOverlapping`
  ;[1 1 1] SetOverlapping
  (`KismetSystemLibrary.PrintString` "This is BP_World Stopping")
  (set `self.Overlap` false))

(event `Enable Combat`
  (if (<= (`KismetMathLibrary.RandomFloatInRange` 0.0 5000.0) 250.0)
    (if (>= (`KismetMathLibrary.RandomFloatInRange` 1000.0 2500.0) 2400.0)
      (`KismetSystemLibrary.PrintString` "EnteringBattle")
      (`self.Set Enemies`)
      (`KismetSystemLibrary.Delay` 2.0)
      (`GameplayStatics.OpenLevel` "Minimal_Default"))))

(event `Set Enemies`
  (bind _asinstance_game (cast `/Game/Blueprints/Instance_Game` (`GameplayStatics.GetGameInstance`)))
  (set `/Game/Blueprints/Instance_Game.Enemy1` (`KismetArrayLibrary.Array_Get` (`self.CurrentEnemies`) (`KismetMathLibrary.RandomInteger` 2)) _asinstance_game)
  (set `/Game/Blueprints/Instance_Game.Enemy2` (`KismetArrayLibrary.Array_Get` (`self.CurrentEnemies`) (`KismetMathLibrary.RandomInteger` 2)) _asinstance_game)
  (set `/Game/Blueprints/Instance_Game.Enemy3` (`KismetArrayLibrary.Array_Get` (`self.CurrentEnemies`) (`KismetMathLibrary.RandomInteger` 2)) _asinstance_game))

(fn `UserConstructionScript`)