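; BP_AI is a combat character with health, stat-scaled damage, a standard attack and a fire attack.
; StandardAttack moves to the target, applies damage after a delay, then returns to the starting spot and rotation, while FireAttack damages at range with an explosion.
; Taking damage briefly shows a floating-text widget, starts a timer turning it toward a BP_Hero attacker, and at zero health sets IsDead and disables movement.
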(event `FireAttack`
  (params (`Target Actor` :type "Actor Object Reference"))
  (`GameplayStatics.SpawnEmitterAtLocation` "/Game/StarterContent/Particles/P_Explosion.P_Explosion" (`self.K2_GetActorLocation` `Target Actor`))
  (`GameplayStatics.ApplyDamage` `Target Actor` (`self.Damage`)))

(event `StandardAttack`
  (params (TargetActor :type "Actor Object Reference"))
  ;[1 1 1] Srandard Attack
  (set `self.Current Rotation` (`self.K2_GetActorRotation`))
  (set `self.Current Location` (`self.K2_GetActorLocation`))
  (`/Engine/EditorBlueprintResources/StandardMacros.IsValid` TargetActor
    (:`Is Valid`
      (`|AIMoveTo` self (0.0 0.0 0.0) TargetActor
        (:`OnSuccess`
          (`KismetSystemLibrary.Delay` 1.5)
          (`GameplayStatics.ApplyDamage` TargetActor (`self.Damage`))
          (`KismetSystemLibrary.Delay` 1.0)
          (`SkeletalMeshComponent.SetAnimationMode` (`self.Mesh`) "AnimationBlueprint")
          (`|AIMoveTo` self (`self.Current Location`)
            (:`OnSuccess`
              (`self.SetActorRotation` (`self.Current Rotation`)))))))))

(event `self.Collision.OnComponentBeginOverlap`
  (params (OtherActor :type "Actor Object Reference") (OtherComp :type "PrimitiveComponent Object Reference") (OtherBodyIndex :type Integer) (bFromSweep :type Boolean) (SweepResult :type "HitResult Structure (by ref)"))
  ;[1 1 1] DealDamageOnHandCollision
)

(event `self.ReceiveAnyDamage`
  (params (Damage :type "Float (single-precision)") (DamageType :type "DamageType Object Reference") (InstigatedBy :type "Controller Object Reference") (DamageCauser :type "Actor Object Reference"))
  ;[1 1 1] Deal Damage and Set dead
  (`SceneComponent.SetHiddenInGame` (`self.Widget`) false false)
  (set `self.Enemy` DamageCauser)
  (`KismetSystemLibrary.K2_SetTimer` null "FollowCharacter" 0.01 true)
  (bind _output_get (set `self.Health` (`KismetMathLibrary.FClamp` (- (`self.Health`) Damage) (`self.HealthMin`) (`self.HealthMax`))))
  (if (<= _output_get 0.0)
    (set `self.IsDead?` true)
    (`CharacterMovementComponent.DisableMovement` (`self.CharacterMovement`)))
  (`KismetSystemLibrary.Delay` 1.0)
  (`SceneComponent.SetHiddenInGame` (`self.Widget`) true false))

(event `self.ReceiveBeginPlay`
  ;[1 1 1] Event Begin Play
  (`self.Calculate Damage`)
  (bind _asfloating_text (cast `/Game/UI/FloatingText` (`WidgetComponent.GetUserWidgetObject` (`self.Widget`))))
  (set `/Game/UI/FloatingText.Actor Ref` self _asfloating_text)
  (set `/Game/UI/FloatingText.FloatDamage` (`self.Damage`) _asfloating_text))

(event `Calculate Damage`
  ;[1 1 1] Calcilate Damage
  (set `self.Damage` (* (/ (+ (`KismetArrayLibrary.Array_Get` (`self.Stats`)) 100.0) 100.0) (`self.BaseDamage`))))

(fn `FollowCharacter`
  (cast `/Game/Blueprints/BP_Hero` (`self.Enemy`))
  (`SceneComponent.K2_SetWorldRotation` (`self.Widget`) (`KismetMathLibrary.MakeRotator` (.roll (`SceneComponent.K2_GetComponentRotation` (`self.Widget`))) (.pitch (`KismetMathLibrary.FindLookAtRotation` (`self.K2_GetActorLocation`) (`self.K2_GetActorLocation` (`self.Enemy`)))) (.yaw (`KismetMathLibrary.FindLookAtRotation` (`self.K2_GetActorLocation`) (`self.K2_GetActorLocation` (`self.Enemy`))))) false false))

(fn `UserConstructionScript`)