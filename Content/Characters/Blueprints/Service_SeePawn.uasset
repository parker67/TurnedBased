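; Behavior tree service for Mixamo AI characters that copies perception and state into the blackboard on each AI tick.
; It caches the controlled Mixamo and mirrors its SeePawn flag.
; While PawnSeen is valid, it stores that pawn as the player if unset (FirstPersonCharacter only, despite the ThirdPersonPlayerKey name) and updates distance to the player.
; The dead flag is written only on that seen-pawn path, once Mixamo is dead.
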(event `self.ReceiveTickAI`
  (params (OwnerController :type "AIController Object Reference") (ControlledPawn :type "Pawn Object Reference") (DeltaSeconds :type "Float (single-precision)"))
  (bind _thirdpersonplayerkey (`self.ThirdPersonPlayerKey`))
  (bind _isdead_ (`/Game/Characters/Blueprints/Mixamo.IsDead?` (`self.Mixamo`)))
  (`/Engine/EditorBlueprintResources/StandardMacros.IsValid` (`self.Mixamo`)
    (:`Is Valid`
      _)
    (:`Is Not Valid`
      (bind _asmixamo (cast `/Game/Characters/Blueprints/Mixamo` ControlledPawn))
      (set `self.Mixamo` _asmixamo)))
  (`BTFunctionLibrary.SetBlackboardValueAsBool` (`self.SeePawnKey`) (`/Game/Characters/Blueprints/Mixamo.SeePawn` _asmixamo))
  (bind _pawnseen (`/Game/Characters/Blueprints/Mixamo.PawnSeen` _asmixamo))
  (`/Engine/EditorBlueprintResources/StandardMacros.IsValid` _pawnseen
    (:`Is Valid`
      (`/Engine/EditorBlueprintResources/StandardMacros.IsValid` (`BTFunctionLibrary.GetBlackboardValueAsActor` (`self.ThirdPersonPlayerKey`))
        (:`Is Valid`
          _)
        (:`Is Not Valid`
          (bind _asfirst_person_character (cast `/Game/FirstPersonBP/Blueprints/FirstPersonCharacter` _pawnseen))
          (`BTFunctionLibrary.SetBlackboardValueAsObject` _thirdpersonplayerkey _asfirst_person_character)))
      (`BTFunctionLibrary.SetBlackboardValueAsFloat` (`self.DistanceToPlayer`) (`KismetMathLibrary.VSize` (- (`Actor.K2_GetActorLocation` (`BTFunctionLibrary.GetBlackboardValueAsActor` _thirdpersonplayerkey)) (`Actor.K2_GetActorLocation` ControlledPawn))))
      (if _isdead_
        (`BTFunctionLibrary.SetBlackboardValueAsBool` (`self.IsDeadKey`) _isdead_)))))